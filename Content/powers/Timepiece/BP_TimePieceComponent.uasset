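; Timepiece power component that shifts its owner between two vertically stacked height bands in the level.
; On activation it stores the owner's current Z, fires the start VFX event, then moves the owner.
; The move keeps X and Y and toggles Z between fixed low and high heights based on a threshold, without a sweep.
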(event EventBeginPlay
  (|CallParentFunction))

(event EventPowerActivate
  (bind _returnvalue (Components|GetOwner))
  (bind _returnvalue_2 (Transformation|GetActorLocation _returnvalue))
  (Variables|Default|SetDeltaZ (.z _returnvalue_2))
  (CallFunction|EventStartVFX)
  (Transformation|SetActorLocation (Components|GetOwner) (Math|Vector|MakeVector (.x _returnvalue_2) (.y _returnvalue_2) (Math|Float|SelectFloat 1e+02 1.01e+04 (>= (Variables|Default|GetDeltaZ) 1e+04))) false false))