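; Blink power that moves its owner to an aimed spot, climbing onto low enough ledges.
; While targeting, a looping timer updates a spawned BP_BlinkTargetDisplay, showing direction pointers for scalable walls.
; A camera-aimed sphere trace finds the spot, a downward trace lowers it, and further traces check wall top and headroom.
; Activation starts VFX, then MoveComponentTo slides the root there and, if scalable, onto the wall.
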(event EventBeginPlay
  (bind _returnvalue (Components|GetOwner))
  ;[1 1 1] Begin Play
  (|CallParentFunction)
  (Utilities|IsValid _returnvalue
    (:Is%20Valid
      (bind _returnvalue_2 (Game|SpawnActorfromClass "/Game/powers/Blink/BP_BlinkTargetDisplay.BP_BlinkTargetDisplay_C" (Transformation|GetActorTransform _returnvalue) "AlwaysSpawn" 0 0))
      (Variables|Default|SetBlinkTargetDisplay _returnvalue_2))
    (:Is%20Not%20Valid
      (Development|PrintString "FAILED TO GET OWNER"))))

(event EventPowerActivate
  ;[1 1 1] Ability Activated
  (if (not (Variables|Default|GetIsBlinking))
    (Variables|Default|SetIsBlinking true)
    (bind (_outscalablelocation _outcanscalewall_ _outblockinghit _outtargetdisplaylocation) (CallFunction|CalculateBlinkTargetData))
    (Utilities|FlowControl|Sequence
      (:then_0
        (CallFunction|EventStartVFX))
      (:then_1
        (bind (_outroot_component _outrelative_rotation) (CallFunction|GetOwnerRootComponentData))
        (Components|MoveComponentTo _outroot_component (+ _outtargetdisplaylocation "0, 0,100.000000") _outrelative_rotation false false (Variables|Default|GetPowerTime) false)
        (if (and _outcanscalewall_ _outblockinghit)
          (bind (_outroot_component_2 _outrelative_rotation_2) (CallFunction|GetOwnerRootComponentData))
          (Components|MoveComponentTo _outroot_component_2 _outscalablelocation _outrelative_rotation_2 false false (Variables|Settings|GetWallScalingTime) false))
        (CallFunction|PowerExecutionComplete)))))

(event EventPowerExecutionComplete
  ;[1 1 1] Execution complete
  (Variables|Default|SetIsBlinking false))

(event EventTargetActivated
  ;[0.03729 0.1014 0.3021] Target
  (if (not (Variables|Default|GetIsBlinking))
    (if (not (CallFunction|IsTargetActivated?))
      (Default|EventEnableBlinkTargetDisplay (Variables|Default|GetBlinkTargetDisplay))
      (CallFunction|UpdateTarget)
      (bind _returnvalue (Utilities|Time|SetTimerbyEvent (delegate EventUpdateTarget) (Variables|Default|GetTargetUpdateInterval) true))
      (Variables|Default|SetTargetTimerHandle _returnvalue))))

(event EventTargetConfirmed
  ;[0.03729 0.1014 0.3021] Target
  (if (CallFunction|IsTargetActivated?)
    (CallFunction|TargetDeactivated)
    (CallFunction|PowerActivate)))

(event EventTargetDeactivated
  ;[0.03729 0.1014 0.3021] Target
  (Utilities|Time|ClearandInvalidateTimerbyHandle (Variables|Default|GetTargetTimerHandle))
  (Default|EventDisableBlinkTargetDisplay (Variables|Default|GetBlinkTargetDisplay)))

(event EventUpdateTarget
  ;[0.03729 0.1014 0.3021] Target
  (bind (_outscalablelocation _outcanscalewall_ _outblockinghit _outtargetdisplaylocation _traceimpactnormal) (CallFunction|CalculateBlinkTargetData))
  (CallFunction|UpdateTargetDisplayLocation _outtargetdisplaylocation _outcanscalewall_ _traceimpactnormal))

(fn CalculateTargetDisplayLocation
  (params (AimTraceHit :type Boolean) (AimTraceHitLocation :type Vector) (AimTraceEndLocation :type Vector))
  (if AimTraceHit
    (LocalVariables|SetLocAimTargetLocation AimTraceHitLocation)
    (else
      (LocalVariables|SetLocAimTargetLocation AimTraceEndLocation)))
  (bind _outhit (Collision|LineTraceByChannel (LocalVariables|GetLocAimTargetLocation) (+ (LocalVariables|GetLocAimTargetLocation) (Math|Vector|MakeVector 0.0 0.0 (* (Variables|Settings|GetCollisionCheckHalfHeight) -1.0))) "TraceTypeQuery1" false 0 "None"))
  (if (.bBlockingHit (Collision|BreakHitResult _outhit))
    (return (.Location (Collision|BreakHitResult _outhit)))
    (else
      (return (.TraceEnd (Collision|BreakHitResult _outhit))))))

(fn EvaluateWallScalingConditions
  (params (AimtraceImpactPoint :type Vector) (AimtraceImpactNormal :type Vector))
  (bind _returnvalue (Math|Vector|Normalize AimtraceImpactNormal))
  (bind _collisioncheckradius (Variables|Settings|GetCollisionCheckRadius))
  (bind _returnvalue_2 (* _collisioncheckradius -1.21))
  (bind _returnvalue_3 (* _returnvalue _returnvalue_2))
  (bind _returnvalue_4 (+ AimtraceImpactPoint _returnvalue_3))
  (if (> (.Z (Math|Vector|BreakVector AimtraceImpactNormal)) 0.1)
    (return "0, 0, 0" false)
    (else
      (bind (_outhit _returnvalue_5) (Collision|LineTraceByChannel (+ _returnvalue_4 (Math|Vector|MakeVector 0.0 0.0 (* (Variables|Settings|GetCollisionCheckHalfHeight) 2.0))) _returnvalue_4 "TraceTypeQuery1" false 0 "None"))
      (if _returnvalue_5
        (if (CallFunction|IsWithingRangeAlongZAxis? (.ImpactPoint (Collision|BreakHitResult _outhit)) (.TraceEnd (Collision|BreakHitResult _outhit)) (Variables|Settings|GetCollisionCheckHalfHeight))
          (bind (_outblockingobjectdetected _outscalablelocation) (CallFunction|ValidateFreeSpaceAboveWall (.ImpactPoint (Collision|BreakHitResult _outhit))))
          (if _outblockingobjectdetected
            (return "0, 0, 0" false)
            (else
              (return _outscalablelocation true)))
          (else
            (return "0, 0, 0" false)))
        (else
          (return "0, 0, 0" false))))))

(fn ValidateFreeSpaceAboveWall
  (params (SurfaceLocationAboveWall :type Vector))
  (bind _outhit (Collision|SphereTraceByChannel (+ SurfaceLocationAboveWall (Math|Vector|MakeVector 0.0 0.0 (+ (Variables|Settings|GetCollisionCheckRadius) 1.0))) (+ SurfaceLocationAboveWall (Math|Vector|MakeVector 0.0 0.0 (* (- (Variables|Settings|GetCollisionCheckHalfHeight) (Variables|Settings|GetCollisionCheckRadius)) 2.0))) (Variables|Settings|GetCollisionCheckRadius) "TraceTypeQuery1" false 0 "None"))
  (return (.bBlockingHit (Collision|BreakHitResult _outhit)) (+ SurfaceLocationAboveWall (Math|Vector|MakeVector 0.0 0.0 (Variables|Settings|GetCollisionCheckHalfHeight)))))

(fn PerformSphereTracetoAimLocation
  (bind _returnvalue (Components|GetOwner))
  (bind _cameracomp (CallFunction|BPIRetrieveCameraComp))
  (bind _outhit (Collision|SphereTraceByChannel (+ (Transformation|GetActorLocation _returnvalue) (* (Transformation|GetActorForwardVector _returnvalue) 5.0)) (+ (Transformation|GetWorldLocation _cameracomp) (* (Math|Vector|GetForwardVector _cameracomp) (Variables|Settings|GetTargetingRange))) (Variables|Settings|GetCollisionCheckRadius) "TraceTypeQuery1" false 0 "None"))
  (return (.bBlockingHit (Collision|BreakHitResult _outhit)) (.ImpactPoint (Collision|BreakHitResult _outhit)) (.ImpactNormal (Collision|BreakHitResult _outhit)) (.Location (Collision|BreakHitResult _outhit)) (.TraceEnd (Collision|BreakHitResult _outhit))))

(fn CalculateBlinkTargetData
  (bind (_outbblockinghit _outimpactpoint _outimpactnormal _outlocation _outtraceend) (CallFunction|PerformSphereTracetoAimLocation))
  (bind (_outscalablelocation _outcanscalewall) (CallFunction|EvaluateWallScalingConditions _outimpactpoint _outimpactnormal))
  (return _outscalablelocation _outcanscalewall _outbblockinghit (CallFunction|CalculateTargetDisplayLocation _outbblockinghit _outlocation _outtraceend) _outimpactnormal))

(fn IsWithingRangeAlongZAxis?
  (params (Location1 :type Vector) (Location2 :type Vector) (Range :type Float%20%28single-precision%29))
  (return (<= (- (.Z (Math|Vector|BreakVector Location1)) (.Z (Math|Vector|BreakVector Location2))) Range)))

(fn UpdateTargetDisplayLocation
  (params (TargetDisplayLocation :type Vector) (DisplayWallScalingDirection? :type Boolean) (AimTraceImpactNormal :type Vector))
  (bind _blinktargetdisplay (Variables|Default|GetBlinkTargetDisplay))
  (bind _blinktargetdisplay_2 (Variables|Default|GetBlinkTargetDisplay))
  (Utilities|IsValid _blinktargetdisplay_2
    (:Is%20Valid
      (Transformation|SetActorLocation _blinktargetdisplay_2 TargetDisplayLocation false false)
      (if DisplayWallScalingDirection?
        (Default|DisplayDirectionPointers _blinktargetdisplay AimTraceImpactNormal)
        (else
          (Default|EventHideDirectionPointers _blinktargetdisplay true)))
      (return))
    (:Is%20Not%20Valid
      (Development|PrintString "BLINK TARGET DISPLAY NOT FOUND"))))

(fn GetOwnerRootComponentData
  (bind _returnvalue (Components|GetOwner))
  (bind _rootcomponent (Variables|/Script/Engine.Actor|GetRootComponent _returnvalue))
  (Utilities|IsValid _returnvalue
    (:Is%20Valid
      (return _rootcomponent (Variables|/Script/Engine.SceneComponent|GetRelativeRotation _rootcomponent)))
    (:Is%20Not%20Valid
      (Development|PrintString "FAILED TO GET OWNER"))))