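; Target indicator actor for the Blink power, with two direction pointers that can show a direction at the target.
; It is hidden on construction, and enable and disable events toggle the whole actor's visibility.
; DisplayDirectionPointers rotates both pointers along a given vector and unhides them, while a separate event sets their visibility.
; The alignment helper keeps each pointer's world roll and adds a 90-degree yaw offset.
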(event Custom|EventEnableBlinkTargetDisplay
  (Rendering|SetActorHiddenInGame false))

(event Custom|EventDisableBlinkTargetDisplay
  (Rendering|SetActorHiddenInGame true))

(event Custom|DisplayDirectionPointers
  (params (DirectionVector :type Vector))
  ;[1 1 1] Aligns direction pointers along the desired vector direction & makes them visible in game
  (CallFunction|AlignComponentAlongUnitVector (Variables|Default|GetDirectionPointer1) DirectionVector)
  (CallFunction|AlignComponentAlongUnitVector (Variables|Default|GetDirectionPointer2) DirectionVector)
  (CallFunction|EventHideDirectionPointers false))

(event Custom|EventHideDirectionPointers
  (params (NewHidden :type Boolean))
  ;[1 1 1] Toggle Direction Pointers
  (Development|SetHiddeninGame (Variables|Default|GetDirectionPointer1) NewHidden false)
  (Development|SetHiddeninGame (Variables|Default|GetDirectionPointer2) NewHidden false))

(fn ConstructionScript
  (CallFunction|EventDisableBlinkTargetDisplay))

(fn AlignComponentAlongUnitVector
  (params (CompRef :type Scene%20Component%20Object%20Reference) (UnitVector :type Vector))
  (bind _returnvalue (Math|Conversions|RotationFromXVector UnitVector))
  (bind (_roll _pitch _yaw) (Math|Rotator|BreakRotator _returnvalue))
  (Transformation|SetWorldRotation CompRef (Math|Rotator|MakeRotator (.Roll (Math|Rotator|BreakRotator (Transformation|GetWorldRotation CompRef))) _pitch (+ _yaw 9e+01)) false false)
  (return))