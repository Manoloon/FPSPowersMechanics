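; Base actor component for powers, exposing empty activation, targeting and completion events to override.
; It caches the owner camera's default FOV on BeginPlay and reports whether targeting is active by checking a timer handle.
; Its start-VFX event runs a looping timer that scales FOV by a float curve over the power's duration, advancing elapsed time in fixed steps.
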(event Custom|Event_StartVFX
  ;[1 1 1] FOv Change and vfx on activation
  (Variables|Default|SetFOVTimeSinceActivation 0.0)
  (bind _returnvalue (Utilities|Time|SetTimerbyEvent (delegate Custom|Event_UpdateFOV) (Variables|Settings|GetFOVUpdateTimerInterval) true))
  (Variables|Default|SetUpdateFOVTimerHandle _returnvalue))

(event Custom|PowerExecutionComplete
  ;[0.2956 1 0.02604] Event for override
)

(event Custom|Event_UpdateFOV
  ;[1 1 1] FOv Change and vfx on activation
  (if (< (+ (Variables|Default|GetFOVTimeSinceActivation) 0.01) (Variables|Settings|GetPowerTime))
    (Variables|Default|SetFOVTimeSinceActivation (+ (Variables|Default|GetFOVTimeSinceActivation) 0.01))
    (else
      (Variables|Default|SetFOVTimeSinceActivation (Variables|Settings|GetPowerTime))
      (Utilities|Time|ClearandInvalidateTimerbyHandle (Variables|Default|GetUpdateFOVTimerHandle))))
  (bind _cameracomp (CallFunction|BPIRetrieveCameraComp))
  (if (Utilities|IsValid _cameracomp)
    (bind _fovmultipliercurve (Variables|Settings|GetFOVMultiplierCurve)
      (:then
        (Camera|SetFieldOfView _cameracomp (* (Variables|Default|GetDefaultFOV) (Math|Curves|GetFloatValue _fovmultipliercurve (Variables|Default|GetFOVTimeSinceActivation)))))
      (:else))
    (else
      (Development|PrintString "No Valid camera"))))

(event Custom|PowerActivate
  ;[0.2956 1 0.02604] Event for override
)

(event Custom|TargetActivated
  ;[0.2956 1 0.02604] Event for override
)

(event Custom|UpdateTarget
  ;[0.2956 1 0.02604] Event for override
)

(event Custom|TargetDeactivated
  ;[0.2956 1 0.02604] Event for override
)

(event Custom|TargetConfirmed
  ;[0.2956 1 0.02604] Event for override
)

(event EventBeginPlay
  (bind _cameracomp (CallFunction|BPIRetrieveCameraComp))
  (Variables|Default|SetDefaultFOV (Variables|/Script/Engine.CameraComponent|GetFieldOfView _cameracomp)))

(fn IsTargetActivated?
  (return (Class|KismetSystemLibrary|TimerExistsHandle (Variables|Default|GetTargetTimerHandle))))

(fn BPIRetrieveCameraComp
  (return (Actor|GetComponentbyClass (Components|GetOwner) "/Script/Engine.CameraComponent")))